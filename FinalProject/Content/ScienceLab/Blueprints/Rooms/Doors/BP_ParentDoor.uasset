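; Parent Blueprint for Science Lab doors that handles automatic opening, locking and status lights.
; When AutoDoor is true, collision overlaps toggle AutoOpen and AutoClose and play a swish sound; door movement is not implemented here.
; UnlockDoor and LockDoor set AutoDoor and recolor the Lights array's emissive material parameter green or red.
; BeginPlay turns the lights red without changing AutoDoor, so its default decides whether the door starts locked.
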(event OnComponentEndOverlap(Collision)
  (params (OverlappedComponent :type Primitive%20Component%20Object%20Reference) (OtherActor :type Actor%20Object%20Reference) (OtherComp :type Primitive%20Component%20Object%20Reference) (OtherBodyIndex :type Integer))
  ;[1 1 1] Detect Player
  (if (Variables|ParentDoorVars|GetAutoDoor)
    (Variables|ParentDoorVars|SetAutoClose true)
    (Variables|ParentDoorVars|SetAutoOpen false)
    (Audio|PlaySoundatLocation "/Game/Game/Sounds/SoundEffects/Swish_Cue.Swish_Cue" (Transformation|GetActorLocation) "0, 0, 0" 1.0 1.0 0.0 0 0 0)))

(event OnComponentBeginOverlap(Collision)
  (params (OverlappedComponent :type Primitive%20Component%20Object%20Reference) (OtherActor :type Actor%20Object%20Reference) (OtherComp :type Primitive%20Component%20Object%20Reference) (OtherBodyIndex :type Integer) (bFromSweep :type Boolean) (SweepResult :type Hit%20Result%20Structure%20%28by%20ref%29))
  ;[1 1 1] Detect Player
  (if (Variables|ParentDoorVars|GetAutoDoor)
    (Variables|ParentDoorVars|SetAutoClose false)
    (Variables|ParentDoorVars|SetAutoOpen true)
    (Audio|PlaySoundatLocation "/Game/Game/Sounds/SoundEffects/Swish_Cue.Swish_Cue" (Transformation|GetActorLocation) "0, 0, 0" 1.0 1.0 0.0 0 0 0)))

(event Custom|Unlock%20Door
  ;[1 1 1] Unlock Door
  (Variables|ParentDoorVars|SetAutoDoor true)
  (for _array_element (Variables|ParentDoorVars|GetLights)
    (Rendering|Material|SetVectorParameterValueonMaterials (Actor|GetComponentbyClass _array_element "/Script/Engine.StaticMeshComponent") "Emmisive color" "0.320449,1.000000,0.108294")))

(event Custom|LockDoor
  ;[1 1 1] Lock Door
  (Variables|ParentDoorVars|SetAutoDoor false)
  (for _array_element (Variables|ParentDoorVars|GetLights)
    (Rendering|Material|SetVectorParameterValueonMaterials (Actor|GetComponentbyClass _array_element "/Script/Engine.StaticMeshComponent") "Emmisive color" "1.000000,0.015526, 0")))

(event EventBeginPlay
  ;[1 1 1] Lock Door
  (for _array_element (Variables|ParentDoorVars|GetLights)
    (Rendering|Material|SetVectorParameterValueonMaterials (Actor|GetComponentbyClass _array_element "/Script/Engine.StaticMeshComponent") "Emmisive color" "1.000000,0.015526, 0")))

(fn ConstructionScript)