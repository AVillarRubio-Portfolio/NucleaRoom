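; BP_Locker02 is a science lab locker prop with one hinged door that can be opened and closed.
; OpenLocker and CloseLocker extend their parent versions, setting the door's yaw variable and calling UpdateLocker to snap it into place without animation.
; Both UpdateLocker and the construction script apply that rotation and a shared material to the body and door, so settings also show in the editor.
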(event Custom|UpdateLocker
  ;[1 1 1] Movement
  (Transformation|SetRelativeRotation (Variables|Default|GetLocker02Door01) (Math|Rotator|MakeRotator 0.0 0.0 (Variables|Default|GetDoor01Rotation)) false false)
  ;[1 1 1] Material
  (Rendering|Material|SetMaterial (Variables|Default|Getlocker02) 0 (Variables|Default|GetMaterial)))

(fn ConstructionScript
  ;[1 1 1] Movement
  (Transformation|SetRelativeRotation (Variables|Default|GetLocker02Door01) (Math|Rotator|MakeRotator 0.0 0.0 (Variables|Default|GetDoor01Rotation)) false false)
  ;[1 1 1] Material
  (Rendering|Material|SetMaterial (Variables|Default|Getlocker02) 0 (Variables|Default|GetMaterial)))

(fn CloseLocker
  (|CallParentFunction)
  (Variables|Default|SetDoor01Rotation 0.0)
  (CallFunction|UpdateLocker))

(fn OpenLocker
  (|CallParentFunction)
  (Variables|Default|SetDoor01Rotation 1e+02)
  (CallFunction|UpdateLocker))