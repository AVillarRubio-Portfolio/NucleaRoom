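; Base locker Blueprint for Science Lab furniture, tracking whether the locker is open and whether it is locked.
; InteractLocker does nothing while locked; otherwise it toggles OpenLocker or CloseLocker and plays an unlock sound at the actor's location.
; Lock and Unlock events set the locked flag.
; The open and close functions only set IsOpen, with no visual movement in this class.
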(event Custom|InteractLocker
  ;[1 1 1] Declaracion de los eventos custom
  (if (not (Variables|Default|GetIsLocked))
    (if (Variables|Default|GetIsOpen)
      (CallFunction|CloseLocker)
      (else
        (CallFunction|OpenLocker)))
    (Audio|PlaySoundatLocation "/Game/Game/Sounds/SoundEffects/UnlockLock_01_Cue.UnlockLock_01_Cue" (Transformation|GetActorLocation) "0, 0, 0" 1.0 1.0 0.0 0 0 0)))

(event Custom|Unlock
  ;[1 1 1] Comment
  (Variables|Default|SetIsLocked false))

(event Custom|Lock
  ;[1 1 1] Comment
  (Variables|Default|SetIsLocked true))

(fn ConstructionScript
  (|CallParentFunction))

(fn OpenLocker
  (Variables|Default|SetIsOpen true))

(fn CloseLocker
  (Variables|Default|SetIsOpen false))