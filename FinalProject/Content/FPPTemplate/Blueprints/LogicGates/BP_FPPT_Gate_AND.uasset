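; Logic gate Blueprint that acts as an AND in a power network, active when its power amount is at least two.
; Power updates add or remove activators in an array, whose length replaces a preset starting amount after first use.
; Two input materials light progressively with that count, while parent logic drives the main power material and finished updates propagate to the target actor.
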(event Custom|Update%20Additional%20Powers
  (CallFunction|UpdatePowerMaterial (Variables|Default|GetInPower1%20Material) (Math|Conversions|ToFloat(Boolean) (>= (CallFunction|GetPowerAmount) 1)) (Variables|Default|GetPower%20Type))
  (CallFunction|UpdatePowerMaterial (Variables|Default|GetInPower2%20Material) (Math|Conversions|ToFloat(Boolean) (>= (CallFunction|GetPowerAmount) 2)) (Variables|Default|GetPower%20Type)))

(event EventBeginPlay
  (|CallParentFunction))

(event Collision|EventActorBeginOverlap
  (params (OtherActor :type Actor%20Object%20Reference))
  (|CallParentFunction OtherActor) ; This node is disabled and will not be called.\nDrag off pins to build functionality.
)

(event EventTick
  (params (DeltaSeconds :type Float%20%28single-precision%29))
  (|CallParentFunction DeltaSeconds) ; This node is disabled and will not be called.\nDrag off pins to build functionality.
)

(event EventSetupMaterialOwners
  (Rendering|Material|SetMaterial (Variables|Default|GetEnergySphere) 0 (Variables|Default|GetMain%20Power%20Material))
  (Rendering|Material|SetMaterial (Variables|Default|GetInPower1) 0 (Variables|Default|GetInPower1%20Material))
  (Rendering|Material|SetMaterial (Variables|Default|GetInPower2) 0 (Variables|Default|GetInPower2%20Material)))

(event EventOnUpdatePowerFinished
  (params (Forced :type Boolean))
  (CallFunction|UpdatePoweronTarget Forced (Variables|Default|GetTarget%20Actor) false false))

(event EventOnPowerUpdate
  (params (New%20Active :type Boolean) (Is%20Forced :type Boolean) (Intial%20Actor :type Actor%20Object%20Reference))
  (bind _activator_array (Variables|Default|GetActivator%20Array))
  (if New%20Active
    (Utilities|Array|AddUnique _activator_array Intial%20Actor)
    (else
      (Utilities|Array|RemoveItem _activator_array Intial%20Actor)))
  (Utilities|FlowControl|Sequence
    (:then_0
      (Utilities|FlowControl|DoOnce false
        (:Completed
          (Variables|Default|SetFirstUse false))))
    (:then_1
      (CallFunction|UpdateAdditionalPowers)
      (|CallParentFunction New%20Active Is%20Forced Intial%20Actor))))

(event EventRunConstructionScripts
  (Variables|Default|SetActive (CallFunction|GetActiveStatus))
  (|CallParentFunction))

(fn ConstructionScript
  (CallFunction|SetupAdditionalPower)
  (|CallParentFunction))

(fn SetupAdditionalPower
  (bind _power_material_new (CallFunction|MakeNewPowerMaterial (>= (CallFunction|GetPowerAmount) 1)))
  (Variables|Default|SetInPower1%20Material _power_material_new)
  (bind _power_material_new_2 (CallFunction|MakeNewPowerMaterial (>= (CallFunction|GetPowerAmount) 2)))
  (Variables|Default|SetInPower2%20Material _power_material_new_2))

(fn GetPowerAmount
  (return (Math|Integer|SelectInt (Variables|Default|GetCustom%20Power%20Amount) (Utilities|Array|Length (Variables|Default|GetActivator%20Array)) (Variables|Default|GetFirstUse))))

(fn GetActiveStatus
  (return (>= (CallFunction|GetPowerAmount) 2)))