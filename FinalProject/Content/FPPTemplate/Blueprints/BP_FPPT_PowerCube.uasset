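; BP_FPPT_PowerCube is a cube item that carries a power type and active state, which it reports through GetActivatorPowerType.
; SetupMaterialOwners applies the main power material to the Item0 component.
; Hits above a bump speed play a collision sound at the impact point after a short random delay, with volume scaled by velocity.
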(event EventBeginPlay
  (|CallParentFunction))

(event Collision|EventActorBeginOverlap
  (params (OtherActor :type Actor%20Object%20Reference))
  (|CallParentFunction OtherActor) ; This node is disabled and will not be called.\nDrag off pins to build functionality.
)

(event EventSetupMaterialOwners
  (Rendering|Material|SetMaterial (Variables|Default|GetItem_0) 0 (Variables|Default|GetMain%20Power%20Material)))

(event EventTick
  (params (DeltaSeconds :type Float%20%28single-precision%29))
  (|CallParentFunction DeltaSeconds) ; This node is disabled and will not be called.\nDrag off pins to build functionality.
)

(event Collision|EventHit
  (params (MyComp :type Primitive%20Component%20Object%20Reference) (Other :type Actor%20Object%20Reference) (OtherComp :type Primitive%20Component%20Object%20Reference) (bSelfMoved :type Boolean) (HitLocation :type Vector :default "0, 0, 0") (HitNormal :type Vector :default "0, 0, 0") (NormalImpulse :type Vector :default "0, 0, 0") (Hit :type Hit%20Result%20Structure%20%28by%20ref%29))
  (bind _item_0 (Variables|Default|GetItem_0))
  (bind _returnvalue (Transformation|GetComponentVelocity _item_0))
  (bind _returnvalue_2 (Math|Vector|VectorLength _returnvalue))
  ;[1 1 1] Collision Sounds
  (if (> _returnvalue_2 (Variables|Default|GetBumpSpeed))
    (Utilities|FlowControl|Delay (Math|Random|RandomFloatinRange 0.05 0.2))
    (Audio|PlaySoundatLocation (Variables|Default|GetBumpSound) HitLocation "0, 0, 0" (Math|Float|Clamp(Float) (/ _returnvalue_2 1e+03) 0.2 4.0) 1.0 0.0 0 0 0)))

(fn ConstructionScript
  (|CallParentFunction))

(fn GetActivatorPowerType
  (return (Variables|Default|GetPower%20Type) (Variables|Default|GetActive)))