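; Small power switch that turns on while at least one active activator of matching power type, such as a power cube, sits in its trigger.
; Trigger overlaps and a BeginPlay box scan update the activator list, validated through the switch-activator interface.
; List changes drive the inherited power update, which forwards to the target actor when finished.
; When the switch is a child actor of a FuseBox, it also has that box recheck its fuses.
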(event OnComponentBeginOverlap(SwitchTrigger)
  (params (OverlappedComponent :type Primitive%20Component%20Object%20Reference) (OtherActor :type Actor%20Object%20Reference) (OtherComp :type Primitive%20Component%20Object%20Reference) (OtherBodyIndex :type Integer) (bFromSweep :type Boolean) (SweepResult :type Hit%20Result%20Structure%20%28by%20ref%29))
  (Utilities|IsCompatibleActivator OtherActor
    (:True
      (Utilities|Array|AddUnique (Variables|Default|GetOverlappeedActivatorsArray) OtherActor))
    (:False
      _))
  (if (== (Utilities|Array|Length (Variables|Default|GetOverlappeedActivatorsArray)) 0)
    (CallFunction|OnPowerUpdate false false)
    (else
      (CallFunction|OnPowerUpdate true false)))
  (bind _asfuse_box (Utilities|Casting|CastToFuseBox (Actor|GetParentActor)))
  (Default|CheckFuses _asfuse_box))

(event OnComponentEndOverlap(SwitchTrigger)
  (params (OverlappedComponent :type Primitive%20Component%20Object%20Reference) (OtherActor :type Actor%20Object%20Reference) (OtherComp :type Primitive%20Component%20Object%20Reference) (OtherBodyIndex :type Integer))
  (Utilities|IsCompatibleActivator OtherActor
    (:True
      (if (Utilities|Array|ContainsItem (Variables|Default|GetOverlappeedActivatorsArray) OtherActor)
        (Utilities|Array|RemoveItem (Variables|Default|GetOverlappeedActivatorsArray) OtherActor)
        (if (== (Utilities|Array|Length (Variables|Default|GetOverlappeedActivatorsArray)) 0) :!label _label
          (CallFunction|OnPowerUpdate false false)
          (else
            (CallFunction|OnPowerUpdate true false)))
        (bind _asfuse_box (Utilities|Casting|CastToFuseBox (Actor|GetParentActor)))
        (Default|CheckFuses _asfuse_box)))
    (:False
      (goto _label))))

(event EventBeginPlay
  (|CallParentFunction)
  (bind _outactors (Collision|BoxOverlapActors (Transformation|GetWorldLocation (Variables|Default|GetSwitch%20Trigger)) "5.000000,5.000000,5.000000" (Utilities|Array|MakeArray "ObjectTypeQuery2") "/Game/FPPTemplate/Blueprints/BP_FPPT_PowerCube.BP_FPPT_PowerCube_C" :!class /Script/Engine.KismetSystemLibrary))
  (for _array_element _outactors
    (Utilities|IsCompatibleActivator _array_element
      (:True
        (Utilities|Array|AddUnique (Variables|Default|GetOverlappeedActivatorsArray) (stale OnComponentBeginOverlap(SwitchTrigger) OtherActor)))
      (:False
        _))
    (if (== (Utilities|Array|Length (Variables|Default|GetOverlappeedActivatorsArray)) 0)
      (CallFunction|OnPowerUpdate false false)
      (else
        (CallFunction|OnPowerUpdate true false)))
    (bind _asfuse_box (Utilities|Casting|CastToFuseBox (Actor|GetParentActor)))
    (Default|CheckFuses _asfuse_box)))

(event Collision|EventActorBeginOverlap
  (params (OtherActor :type Actor%20Object%20Reference))
  (|CallParentFunction OtherActor) ; This node is disabled and will not be called.\nDrag off pins to build functionality.
)

(event EventTick
  (params (DeltaSeconds :type Float%20%28single-precision%29))
  (|CallParentFunction DeltaSeconds) ; This node is disabled and will not be called.\nDrag off pins to build functionality.
)

(event EventSetupMaterialOwners
  (Rendering|Material|SetMaterial (Variables|Default|GetStaticMesh) 1 (Variables|Default|GetMain%20Power%20Material)))

(event EventOnUpdatePowerFinished
  (params (Forced :type Boolean))
  (CallFunction|UpdatePoweronTarget Forced (Variables|Default|GetTarget%20Actor) false false))

(fn ConstructionScript
  (|CallParentFunction))