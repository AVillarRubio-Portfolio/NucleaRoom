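; Game instance Blueprint that applies the player's display, graphics, audio and mouse settings.
; SetSettings calls events for resolution, quality, volume and sensitivity in turn.
; Resolution and quality run console commands picked from arrays by index, while volume overrides the master sound class through a pushed sound mix.
; Sensitivity casts the current player character to Player and writes scaled X and Y values to it.
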(event Custom|SetResolution
  ;[1 1 1] Set screen Resolution
  (Development|ExecuteConsoleCommand (Utilities|Array|Get(acopy) (Variables|GameOptionsVars|GetResolutionCommands) (Variables|GameOptionsVars|GetResolution)) 0))

(event Custom|SetQuality
  ;[1 1 1] Set graphics Quality
  (Development|ExecuteConsoleCommand (Utilities|Array|Get(acopy) (Variables|GameOptionsVars|GetQualityCommands) (Variables|GameOptionsVars|GetQuality)) 0))

(event Custom|SetVolume
  ;[1 1 1] Set master Volume
  (Audio|SetSoundMixClassOverride "/Game/Game/Sounds/MasterMixSoundClass.MasterMixSoundClass" "/Game/Game/Sounds/MasterSoundClass.MasterSoundClass" (/ (Variables|GameOptionsVars|GetVolume) 1e+02) 1.0 0.0 true)
  (Audio|PushSoundMixModifier "/Game/Game/Sounds/MasterMixSoundClass.MasterMixSoundClass"))

(event Custom|SetSettings
  ;[1 1 1] Set Settings
  (CallFunction|SetResolution)
  (CallFunction|SetQuality)
  (CallFunction|SetVolume)
  (CallFunction|SetSensitivity))

(event Custom|SetSensitivity
  ;[1 1 1] Set Mouse Sensitivity
  (bind _asplayer (Utilities|Casting|CastToPlayer (Game|GetPlayerCharacter 0)))
  (Variables|/Game/Game/Blueprints/Player.Player_C|SetMouseSensitivityX _asplayer (/ (Variables|GameOptionsVars|GetSensitivityX) 5e+01))
  (Variables|/Game/Game/Blueprints/Player.Player_C|SetMouseSensitivityY _asplayer (/ (Variables|GameOptionsVars|GetSensitivityY) 5e+01)))