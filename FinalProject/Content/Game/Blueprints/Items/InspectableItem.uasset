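; InspectableItem is an item actor that the player can inspect and rotate with the mouse.
; StartInspect moves input from the Inspector to the item, and pressing Inspect hands it back and calls UnInspect on the Player.
; While either mouse button is held, mouse axes apply yaw and pitch to the Item component.
; Reset events use rotations cached at BeginPlay, with RestartTransform also teleporting the actor to a given drop location.
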(event Custom|Start%20Inspect
  (params (Inspector :type Pawn%20Object%20Reference))
  (bind _returnvalue (Game|GetPlayerController 0))
  ;[1 1 1] Start/Stop Inspect
  (Input|DisableInput Inspector _returnvalue)
  (Input|EnableInput _returnvalue))

(event Custom|RestartTransform
  (params (Location :type Vector))
  (bind _item (Variables|Default|GetItem))
  ;[1 1 1] Rotate Item
  ;;[1 1 1] Reset full transform when droped
  (Transformation|SetRelativeRotation _item "0, 0, 0" false false)
  (Transformation|SetWorldRotation _item (Variables|InspectableItemVars|GetStartRotation) false false)
  (Transformation|SetActorLocation (Components|GetOwner _item) Location false false))

(event Custom|ResetItemRotation
  ;[1 1 1] Rotate Item
  ;;[1 1 1] Reset only item rotation
  (Transformation|SetRelativeRotation (Variables|Default|GetItem) (Variables|InspectableItemVars|GetStartRelativeRotation) false false))

(event EventBeginPlay
  (bind _item (Variables|Default|GetItem))
  ;[1 1 1] Set up initializing variables
  (|CallParentFunction)
  (Variables|InspectableItemVars|SetStartRotation (Transformation|GetWorldRotation _item))
  (Variables|InspectableItemVars|SetStartLocation (Variables|/Script/Engine.SceneComponent|GetRelativeLocation _item))
  (Variables|InspectableItemVars|SetStartRelativeRotation (Variables|/Script/Engine.SceneComponent|GetRelativeRotation _item)))

(event Collision|EventActorBeginOverlap
  (params (OtherActor :type Actor%20Object%20Reference))
  ;[1 1 1] Call parent methods
  (|CallParentFunction OtherActor))

(event EventTick
  (params (DeltaSeconds :type Float%20%28single-precision%29))
  ;[1 1 1] Call parent methods
  (|CallParentFunction DeltaSeconds))

(event Input|ActionEvents|InputActionInspect
  (params (Key :type Key%20Structure :default "None"))
  (bind _returnvalue (Game|GetPlayerController 0))
  ;[1 1 1] Start/Stop Inspect
  (:Pressed
    (Input|DisableInput _returnvalue)
    (Input|EnableInput (stale Custom|Start%20Inspect Inspector) _returnvalue)
    (bind _asplayer (Utilities|Casting|CastToPlayer (stale Custom|Start%20Inspect Inspector)))
    (Default|UnInspect _asplayer)))

(event Input|MouseEvents|MouseX
  (params (AxisValue :type Float%20%28single-precision%29))
  (bind _returnvalue (Game|GetPlayerController 0))
  ;[1 1 1] Rotate Item
  (if (or (Game|Player|IsInputKeyDown _returnvalue "LeftMouseButton") (Game|Player|IsInputKeyDown _returnvalue "RightMouseButton"))
    (Transformation|SetRelativeRotation (Variables|Default|GetItem) (Math|Rotator|CombineRotators (Variables|/Script/Engine.SceneComponent|GetRelativeRotation (Variables|Default|GetItem)) (Math|Rotator|MakeRotator 0.0 0.0 (* AxisValue -1.0))) false false)))

(event Input|MouseEvents|MouseY
  (params (AxisValue :type Float%20%28single-precision%29))
  (bind _returnvalue (Game|GetPlayerController 0))
  ;[1 1 1] Rotate Item
  (if (or (Game|Player|IsInputKeyDown _returnvalue "LeftMouseButton") (Game|Player|IsInputKeyDown _returnvalue "RightMouseButton"))
    (Transformation|SetRelativeRotation (Variables|Default|GetItem) (Math|Rotator|CombineRotators (Variables|/Script/Engine.SceneComponent|GetRelativeRotation (Variables|Default|GetItem)) (Math|Rotator|MakeRotator 0.0 (* AxisValue -1.0) 0.0)) false false)))

(fn ConstructionScript
  (|CallParentFunction))