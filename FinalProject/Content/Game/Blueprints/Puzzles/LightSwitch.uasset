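; Light switch puzzle actor that turns a set of linked lights on or off and plays a matching sound.
; At BeginPlay it takes the light list from its parent Switch actor and applies the initial on/off state to each light.
; On and off events toggle every valid light, update the state and swap audio playback.
; The construction script previews the state on the lights and creates hidden audio components for both sounds.
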(event Custom|Switch%20Lights%20On
  ;[1 1 1] Switch lights On/Off on switch interacted
  (for _array_element (Variables|SwitchVars|GetLights)
    (Utilities|IsValid _array_element
      (:Is%20Valid
        (Default|Turnon _array_element))))
  (Variables|SwitchVars|SetSwitch%20On true)
  (Audio|Components|Audio|Stop (Variables|Default|GetAudio%20TurnOff%20Component))
  (Audio|Components|Audio|Play (Variables|Default|GetAudio%20TurnOn%20Component) 0.0))

(event Custom|Switch%20Lights%20Off
  ;[1 1 1] Switch lights On/Off on switch interacted
  (for _array_element (Variables|SwitchVars|GetLights)
    (Utilities|IsValid _array_element
      (:Is%20Valid
        (Default|TurnOff _array_element))))
  (Variables|SwitchVars|SetSwitch%20On false)
  (Audio|Components|Audio|Stop (Variables|Default|GetAudio%20TurnOn%20Component))
  (Audio|Components|Audio|Play (Variables|Default|GetAudio%20TurnOff%20Component) 0.0))

(event EventBeginPlay
  ;[1 1 1] Init switch and linked lights
  (Audio|Components|Audio|Stop (Variables|Default|GetAudio%20TurnOff%20Component))
  (bind _asswitch (Utilities|Casting|CastToSwitch (Actor|GetParentActor)))
  (bind _output_get (Variables|SwitchVars|SetLights (Variables|/Game/Game/Blueprints/Puzzles/Switch.Switch_C|GetLights _asswitch)))
  (for _array_element _output_get
    (Utilities|IsValid _array_element
      (:Is%20Valid
        (Variables|/Game/InteractiveLights/Blueprints/BaseElements/Light_Base.Light_Base_C|SetEnabled _array_element (Variables|SwitchVars|GetSwitch%20On))
        (Default|Constructor _array_element)))))

(fn ConstructionScript
  (for _array_element (Variables|SwitchVars|GetLights)
    (if (Variables|SwitchVars|GetSwitch%20On)
      (Variables|/Game/InteractiveLights/Blueprints/BaseElements/Light_Base.Light_Base_C|SetEnabled _array_element true)
      (else
        (Variables|/Game/InteractiveLights/Blueprints/BaseElements/Light_Base.Light_Base_C|SetEnabled _array_element false)))
    (Default|Constructor _array_element))
  (CallFunction|SetupAudio))

(fn SetupAudio
  (bind _box (Variables|Default|GetBox))
  (bind _returnvalue (Transformation|GetRelativeTransform _box))
  (Utilities|FlowControl|Sequence
    (:then_0
      (Utilities|IsValid (Variables|Default|GetAudio%20TurnOn%20Component)
        (:Is%20Valid
          _)
        (:Is%20Not%20Valid
          (bind _returnvalue_2 (AddComponent|AddAudioComponent false _returnvalue))
          (bind _output_get (Variables|Default|SetAudio%20TurnOn%20Component _returnvalue_2))))
      (Audio|Components|Audio|SetSound _output_get (Variables|SwitchVars|GetSwitch%20On%20Sound)))
    (:then_1
      (Utilities|IsValid (Variables|Default|GetAudio%20TurnOff%20Component)
        (:Is%20Valid
          _)
        (:Is%20Not%20Valid
          (bind _returnvalue_3 (AddComponent|AddAudioComponent false _returnvalue))
          (bind _output_get_2 (Variables|Default|SetAudio%20TurnOff%20Component _returnvalue_3))))
      (Audio|Components|Audio|SetSound _output_get_2 (Variables|SwitchVars|GetSwitch%20Off%20Sound)))
    (:then_2
      (Rendering|SetVisibility (Variables|Default|GetAudio%20TurnOn%20Component) false true))))