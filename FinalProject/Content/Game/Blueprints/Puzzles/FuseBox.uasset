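; FuseBox is a puzzle actor that locks or unlocks a linked Target door based on the state of its fuse switches.
; CheckFuses recursively gathers child actors, casts them to BP_FPPT_PowerSwitchSmall and ANDs their Active flags.
; If Target is valid, it unlocks the door when the combined result is true and locks it otherwise.
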(event Custom|CheckFuses
  (bind _target (Variables|Fuseboxvars|GetTarget))
  ;[1 1 1] When all fuses are powering on, unlocks the linked door
  (Variables|Fuseboxvars|SetUnlockTarget true)
  (for _array_element (Actor|GetAllChildActors true)
    (bind _asbp_fppt_power_switch_small (Utilities|Casting|CastToBP_FPPT_PowerSwitchSmall _array_element))
    (Variables|Fuseboxvars|SetUnlockTarget (and (Variables|/Game/FPPTemplate/Blueprints/Core/BP_FPPT_Base.BP_FPPT_Base_C|GetActive _asbp_fppt_power_switch_small) (Variables|Fuseboxvars|GetUnlockTarget))))
  (Utilities|IsValid _target
    (:Is%20Valid
      (if (Variables|Fuseboxvars|GetUnlockTarget)
        (Default|UnlockDoor _target)
        (else
          (Default|LockDoor _target))))))

(event EventBeginPlay
  ;[1 1 1] Call parent methods
  (|CallParentFunction))

(fn ConstructionScript
  (|CallParentFunction))