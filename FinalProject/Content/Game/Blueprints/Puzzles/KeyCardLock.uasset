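; Key card lock puzzle actor that accepts one assigned Key item and unlocks a linked Door.
; On activation with the matching key, it plays a confirm beep, detaches the item, aligns it and resets its inspect rotation.
; A CardPass timeline swipes the card between two scene points, then after a short delay destroys it and calls UnlockDoor.
; Any other item only triggers an error beep.
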(event Custom|OnKeyCardLockActivated
  (params (UsedActor :type Actor%20Object%20Reference))
  (bind _returnvalue (Transformation|GetActorLocation))
  (bind _key (Variables|KeyCardVars|GetKey))
  (bind _passanimstart (Variables|Default|GetPassAnimStart))
  ;[1 1 1] Check if key is correct, feedback, destroy key, open linked door
  (if (== UsedActor _key)
    (Audio|PlaySoundatLocation "/Game/Game/Sounds/SoundEffects/CorrectBeep_01_Cue.CorrectBeep_01_Cue" _returnvalue "0, 0, 0" 1.0 1.0 0.0 0 0 0)
    (Utilities|FlowControl|Sequence
      (:then_0
        (Transformation|DetachFromActor UsedActor "KeepWorld" "KeepWorld" "KeepWorld")
        (Transformation|SetActorRotation UsedActor (Transformation|GetWorldRotation _passanimstart))
        (bind _asinspectable_item (Utilities|Casting|CastToInspectableItem UsedActor))
        (Default|ResetItemRotation _asinspectable_item))
      (:then_1
        (bind _lerpalpha (Timeline|CardPass Play)
          (:Update
            (Transformation|SetActorLocation _key (Math|Vector|Lerp(Vector) (Transformation|GetWorldLocation _passanimstart) (Transformation|GetWorldLocation (Variables|Default|GetPassAnimEnd)) _lerpalpha) false false))
          (:Finished
            (Utilities|FlowControl|Delay 0.2)
            (Actor|DestroyActor UsedActor)
            (Default|UnlockDoor (Variables|KeyCardVars|GetDoor))))))
    (else
      (Audio|PlaySoundatLocation "/Game/Game/Sounds/SoundEffects/WrongBeep_Cue.WrongBeep_Cue" _returnvalue "0, 0, 0" 1.0 1.0 0.0 0 0 0))))

(event EventBeginPlay
  ;[1 1 1] Call parent methods
  (|CallParentFunction) ; This node is disabled and will not be called.\nDrag off pins to build functionality.
)

(fn ConstructionScript
  (|CallParentFunction))