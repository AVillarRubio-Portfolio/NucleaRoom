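; Lock puzzle actor that checks whether the item used on it is its assigned Key, rattling a chain sound otherwise.
; On a match it plays an unlock sound, detaches and aligns the key, then chains timelines that slide it between two marker components and roll it.
; After the turn it unlocks the linked TargetLocker and, following a short delay, destroys the key and its own lock components.
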(event Custom|OnLockInteracted
  (params (UsedActor :type Actor%20Object%20Reference))
  (bind _returnvalue (Transformation|GetActorLocation))
  (bind _key (Variables|LockedBoxVars|GetKey))
  (bind _lockpos (Variables|Default|GetLockPos))
  (bind _targetlocker (Variables|LockedBoxVars|GetTargetLocker))
  (bind _returnvalue_2 (Transformation|GetActorRotation _key))
  (bind (_roll _pitch _yaw) (Math|Rotator|BreakRotator _returnvalue_2))
  ;[1 1 1] Check if key is correct, show feedback, destroy key, open linked door
  (if (== UsedActor _key)
    (Audio|PlaySoundatLocation "/Game/Game/Sounds/SoundEffects/UnlockLock_02_Cue.UnlockLock_02_Cue" _returnvalue "0, 0, 0" 1.0 1.0 0.0 0 0 0)
    (Utilities|FlowControl|Sequence
      (:then_0
        (Transformation|DetachFromActor UsedActor "KeepWorld" "KeepWorld" "KeepWorld")
        (Transformation|SetActorRotation UsedActor (Transformation|GetWorldRotation _lockpos))
        (bind _asinspectable_item (Utilities|Casting|CastToInspectableItem UsedActor))
        (Default|ResetItemRotation _asinspectable_item))
      (:then_1
        (bind _lerpalpha (Timeline|MoveKey Play)
          (:Update
            (Transformation|SetActorLocation _key (Math|Vector|Lerp(Vector) (Transformation|GetWorldLocation _lockpos) (Transformation|GetWorldLocation (Variables|Default|GetLockPosEnd)) _lerpalpha) false false))
          (:Finished
            (bind _lerpalpha_2 (Timeline|RotateKey Play)
              (:Update
                (Transformation|SetActorRotation _key (Math|Rotator|MakeRotator _lerpalpha_2 _pitch _yaw)))
              (:Finished
                (Utilities|FlowControl|Sequence
                  (:then_0
                    (Utilities|FlowControl|Delay 0.2)
                    (Actor|DestroyActor UsedActor)
                    (Components|DestroyComponent (Variables|Default|GetLock))
                    (Components|DestroyComponent (Variables|Default|GetLock1))
                    (Components|DestroyComponent (Variables|Default|GetLock2)))
                  (:then_1
                    (Utilities|IsValid _targetlocker
                      (:Is%20Valid
                        (Default|Unlock _targetlocker)))))))))))
    (else
      (Audio|PlaySoundatLocation "/Game/Game/Sounds/SoundEffects/ChainRattle_Cue.ChainRattle_Cue" _returnvalue "0, 0, 0" 1.0 1.0 0.0 0 0 0))))

(event EventBeginPlay
  ;[1 1 1] Call parent method
  (|CallParentFunction) ; This node is disabled and will not be called.\nDrag off pins to build functionality.
)

(fn ConstructionScript
  (|CallParentFunction))