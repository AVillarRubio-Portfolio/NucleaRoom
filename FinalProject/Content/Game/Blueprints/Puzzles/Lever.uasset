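; Puzzle lever that ends a level's red-light alarm state and triggers the win, built as a child Blueprint that calls its parent's events.
; BeginPlay caches the original colors of the referenced lights and turns them red.
; SwitchLever toggles a timeline forward or in reverse to rotate the handle.
; Each timeline update also restores the light colors, stops the sound and calls CallWin after a short delay.
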(event Custom|SwitchLever
  ;[1 1 1] Toggle when interacted
  (Variables|LeverVars|SetOnOff (not (Variables|LeverVars|GetOnOff)))
  (if (Variables|LeverVars|GetOnOff)
    (bind _onmove (Timeline|OnMove Play)
      (:Update
        (Transformation|SetRelativeRotation (Variables|Default|GetLever) (Math|Rotator|Lerp(Rotator) (Variables|LeverVars|GetOff%20Rot) (Variables|LeverVars|GetOn%20Rot) _onmove) false false)
        (CallFunction|ToCalmLevel)
        (Utilities|FlowControl|Delay 0.5)
        (Default|CallWin)))
    (else
      (Timeline|OnMove Reverse))))

(event Custom|toCalmLevel
  ;[1 1 1] Turn the lights blue again
  (for (_array_element _array_index) (Variables|LeverVars|GetLights)
    (Rendering|Components|Light|SetLightColor (Variables|/Script/Engine.Light|GetLightComponent _array_element) (Math|Conversions|ToLinearColor(Color) (Utilities|Array|Get(acopy) (Variables|LeverVars|GetLightsOrigColor) _array_index)) true)
    (Audio|Components|Audio|Stop (Variables|/Script/Engine.AmbientSound|GetAudioComponent (Variables|LeverVars|GetSoundCue)))))

(event EventBeginPlay
  ;[1 1 1] Initial Set up
  (|CallParentFunction)
  (Variables|LeverVars|SetOn%20Rot "0, 0,-40.000000")
  (Variables|LeverVars|SetOff%20Rot "0, 0,40.000000")
  (for _array_element (Variables|LeverVars|GetLights)
    (Utilities|Array|Add (Variables|LeverVars|GetLightsOrigColor) (Math|Conversions|ToColor(LinearColor) (Rendering|Components|Light|GetLightColor (Variables|/Script/Engine.Light|GetLightComponent _array_element))))
    (Rendering|Components|Light|SetLightColor (Variables|/Script/Engine.Light|GetLightComponent _array_element) (Variables|LeverVars|GetRedColor) true)))

(event Collision|EventActorBeginOverlap
  (params (OtherActor :type Actor%20Object%20Reference))
  ;[1 1 1] Call parent methods
  (|CallParentFunction OtherActor))

(event EventTick
  (params (DeltaSeconds :type Float%20%28single-precision%29))
  ;[1 1 1] Call parent methods
  (|CallParentFunction DeltaSeconds))

(fn ConstructionScript)