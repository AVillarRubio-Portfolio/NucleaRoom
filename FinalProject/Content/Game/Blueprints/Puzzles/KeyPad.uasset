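; Keypad puzzle actor that unlocks an assigned door and/or locker when the player enters its secret code.
; ClickNumber reads the digit from the second character of the clicked component's name and appends it to the input.
; At full code length, a match locks further input and unlocks the targets, while a mismatch clears it, each with a beep.
; Two chained timelines press and release each button.
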(event Custom|ClickNumber
  (params (NewParam :type Primitive%20Component%20Object%20Reference))
  (bind _returnvalue (Utilities|String|ToString(Object) NewParam))
  (bind _returnvalue_2 (Transformation|GetActorLocation))
  (bind _targetdoor (Variables|KeypadVars|GetTargetDoor))
  (bind _targetlocker (Variables|KeypadVars|GetTargetLocker))
  (bind _returnvalue_3 (Utilities|String|GetSubstring _returnvalue 1))
  ;[1 1 1] On click number behaviour, check if number correct
  (if (not (Variables|KeypadVars|GetCorrect))
    (if (Class|KismetStringLibrary|IsNumeric _returnvalue_3)
      (CallFunction|ButtonAnim NewParam)
      (Variables|KeypadVars|SetUserInput (Utilities|String|Append (Variables|KeypadVars|GetUserInput) _returnvalue_3))
      (if (== (Utilities|String|Len (Variables|KeypadVars|GetUserInput)) (Utilities|String|Len (Variables|KeypadVars|GetSecretNumber)))
        (if (Utilities|Enum|Equal(Enum) (Variables|KeypadVars|GetUserInput) (Variables|KeypadVars|GetSecretNumber))
          (Variables|KeypadVars|SetCorrect true)
          (Audio|PlaySoundatLocation "/Game/Game/Sounds/SoundEffects/CorrectBeep_01_Cue.CorrectBeep_01_Cue" _returnvalue_2 "0, 0, 0" 1.0 1.0 0.0 0 0 0)
          (Utilities|IsValid _targetdoor
            (:Is%20Valid
              (Default|UnlockDoor _targetdoor))
            (:Is%20Not%20Valid
              _))
          (Utilities|IsValid _targetlocker
            (:Is%20Valid
              (Default|Unlock _targetlocker)))
          (else
            (Variables|KeypadVars|SetUserInput "")
            (Audio|PlaySoundatLocation "/Game/Game/Sounds/SoundEffects/WrongBeep_Cue.WrongBeep_Cue" _returnvalue_2 "0, 0, 0" 1.0 1.0 0.0 0 0 0)))))))

(event Custom|ButtonAnim
  (params (Number :type Primitive%20Component%20Object%20Reference))
  ;[1 1 1] Animate buttons on clicked
  (Audio|PlaySoundatLocation "/Game/Game/Sounds/SoundEffects/Click_01_Cue.Click_01_Cue" (Transformation|GetActorLocation) "0, 0, 0" 1.0 1.0 0.0 0 0 0)
  (Variables|KeypadVars|SetStartButtonLoc (Variables|/Script/Engine.SceneComponent|GetRelativeLocation Number))
  (Variables|KeypadVars|SetEndButtonLoc (- (Variables|KeypadVars|GetStartButtonLoc) "0,1.000000, 0"))
  (bind _buttonmove (Timeline|Click PlayFromStart)
    (:Update
      (Transformation|SetRelativeLocation Number (Math|Vector|Lerp(Vector) (Variables|KeypadVars|GetStartButtonLoc) (Variables|KeypadVars|GetEndButtonLoc) _buttonmove) false false))
    (:Finished
      (bind _buttonmove_2 (Timeline|Click%20Re Play)
        (:Update
          (Transformation|SetRelativeLocation Number (Math|Vector|Lerp(Vector) (Variables|KeypadVars|GetEndButtonLoc) (Variables|KeypadVars|GetStartButtonLoc) _buttonmove_2) false false))))))

(event EventBeginPlay
  ;[1 1 1] Call parent methods
  (|CallParentFunction))

(event Collision|EventActorBeginOverlap
  (params (OtherActor :type Actor%20Object%20Reference))
  ;[1 1 1] Call parent methods
  (|CallParentFunction OtherActor))

(event EventTick
  (params (DeltaSeconds :type Float%20%28single-precision%29))
  ;[1 1 1] Call parent methods
  (|CallParentFunction DeltaSeconds))

(fn ConstructionScript)