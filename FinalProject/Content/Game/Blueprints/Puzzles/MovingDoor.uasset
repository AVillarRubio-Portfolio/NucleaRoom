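; MovingDoor is a puzzle door that slides open when the Player overlaps it and closes when they leave, once it has been unlocked.
; BeginPlay caches the world locations of the open and closed position markers.
; A timeline lerps the visual mesh between those points, playing forward to open and in reverse to close.
; UnlockDoorMovement sets the flag that allows both movements.
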(event Custom|OpenDoor
  ;[1 1 1] Open/Close door
  (if (Variables|DoorVars|GetIsUnlocked)
    (bind _lerpalpha (Timeline|MoveDoor Play)
      (:Update
        (Transformation|SetWorldLocation (Variables|Default|GetVisualMesh) (Math|Vector|Lerp(Vector) (Variables|DoorVars|GetCloseDoorPos) (Variables|DoorVars|GetOpenDoorPos) _lerpalpha) false false)))))

(event Custom|CloseDoor
  ;[1 1 1] Open/Close door
  (if (Variables|DoorVars|GetIsUnlocked)
    (bind _lerpalpha (Timeline|MoveDoor Reverse)
      (:Update
        (Transformation|SetWorldLocation (Variables|Default|GetVisualMesh) (Math|Vector|Lerp(Vector) (Variables|DoorVars|GetCloseDoorPos) (Variables|DoorVars|GetOpenDoorPos) _lerpalpha) false false)))))

(event Custom|UnlockDoorMovement
  ;[1 1 1] Unlock door
  (Variables|DoorVars|SetIsUnlocked true))

(event EventBeginPlay
  ;[1 1 1] Get open/closed positions
  (Variables|DoorVars|SetOpenDoorPos (Transformation|GetWorldLocation (Variables|Default|GetOpenedDoorPos)))
  (Variables|DoorVars|SetCloseDoorPos (Transformation|GetWorldLocation (Variables|Default|GetClosedDoorPos))))

(event Collision|EventActorBeginOverlap
  (params (OtherActor :type Actor%20Object%20Reference))
  ;[1 1 1] Automatic open/close door on proximity
  (Utilities|Casting|CastToPlayer OtherActor)
  (CallFunction|OpenDoor))

(event Collision|EventActorEndOverlap
  (params (OtherActor :type Actor%20Object%20Reference))
  ;[1 1 1] Automatic open/close door on proximity
  (Utilities|Casting|CastToPlayer OtherActor)
  (CallFunction|CloseDoor))

(fn ConstructionScript)