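; Timer Blueprint that runs the game's minutes and seconds countdown and triggers the lose condition at zero.
; While TimerOn is set, Tick feeds a one-second Delay, which paces the countdown because repeat calls are ignored while it waits.
; Each step decrements Seconds, rolling over into Minutes, then calls TimeChanged for UI updates.
; When both values are already zero, it calls Lose instead.
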(event EventTick
  (params (DeltaSeconds :type Float%20%28single-precision%29))
  ;[1 1 1] Timer, when updated every second, sends call for the UI to update, as well as handle game end when reaches 0
  (if (Variables|TimerVars|GetTimerOn)
    (Utilities|FlowControl|Delay 1.0)
    (if (== (Variables|TimerVars|GetSeconds) 0)
      (if (== (Variables|TimerVars|GetMinutes) 0)
        (Default|CallLose)
        (else
          (Variables|TimerVars|SetSeconds 59)
          (Variables|TimerVars|SetMinutes (- (Variables|TimerVars|GetMinutes) 1))
          (Default|CallTimeChanged :!label _label)))
      (else
        (Variables|TimerVars|SetSeconds (- (Variables|TimerVars|GetSeconds) 1))
        (goto _label)))))

(fn ConstructionScript)