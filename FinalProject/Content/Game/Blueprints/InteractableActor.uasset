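; InteractableActor is an actor for interactable objects that shows a white outline when the player looks at it.
; Its Outline and UnOutline events toggle Custom Depth rendering and the stencil value on the Item component and all its descendant static meshes.
; It only sets these render flags, with no look detection, outline drawing or interaction logic in its graphs.
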(event Custom|Outline
  (bind _item (Variables|Default|GetItem))
  ;[1 1 1] Creates white outline around meshes of interactable object when looked at them
  (Utilities|FlowControl|Sequence
    (:then_0
      (Rendering|SetRenderCustomDepth _item true)
      (Rendering|SetCustomDepthStencilValue _item 2))
    (:then_1
      (for _array_element (Components|GetChildrenComponents (Variables|Default|GetItem) true)
        (bind _asstatic_mesh_component (Utilities|Casting|CastToStaticMeshComponent _array_element))
        (Rendering|SetRenderCustomDepth _asstatic_mesh_component true)
        (Rendering|SetCustomDepthStencilValue _asstatic_mesh_component 2)))))

(event Custom|UnOutline
  (bind _item (Variables|Default|GetItem))
  ;[1 1 1] Removes the white outline around meshes of interactable object when looked at them
  (Utilities|FlowControl|Sequence
    (:then_0
      (Rendering|SetRenderCustomDepth _item false)
      (Rendering|SetCustomDepthStencilValue _item 0))
    (:then_1
      (for _array_element (Components|GetChildrenComponents (Variables|Default|GetItem) true)
        (bind _asstatic_mesh_component (Utilities|Casting|CastToStaticMeshComponent _array_element))
        (Rendering|SetRenderCustomDepth _asstatic_mesh_component false)
        (Rendering|SetCustomDepthStencilValue _asstatic_mesh_component 0)))))

(fn ConstructionScript)